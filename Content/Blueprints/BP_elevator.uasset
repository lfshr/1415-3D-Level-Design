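; Elevator Blueprint that moves its Elevator component toward target node actors, starting with FirstStopTarget as set in construction.
; MoveToNode sets a new target and flags it as moving.
; UpdateSpeed accumulates clamped acceleration, and UpdateLocation applies that speed along the look-at direction as a swept step, without delta-time scaling.
; The event graph is inactive, so nothing here calls these functions, and no arrival check exists.
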(event EventBeginPlay)

(event EventActorBeginOverlap
  (params (OtherActor :type Actor%20Object%20Reference)))

(event EventTick
  (params (DeltaSeconds :type Float%20%28single-precision%29)))

(fn ConstructionScript
  (Variables|Default|SettargetNode (Variables|Default|GetfirstStopTarget)))

(fn MovetoNode
  (params (node :type BP%20Elevator%20Node%20Object%20Reference))
  (Variables|Default|SettargetNode node)
  (Variables|Default|Setmoving true))

(fn UpdateSpeed
  (bind _maxspeed (Variables|Default|GetmaxSpeed))
  (Variables|Default|SetcurSpeed (Math|Float|Clamp(Float) (+ (Variables|Default|GetcurSpeed) (Variables|Default|GetaccelSpeed)) (* _maxspeed -1.0) _maxspeed)))

(fn UpdateLocation
  (if (not (== (Variables|Default|GettargetNode) 0))
    (Transformation|SetWorldLocation (Variables|Default|Getelevator) (+ (* (Math|Vector|Normalize (Math|Vector|GetForwardVector (Math|Rotator|FindLookatRotation (Transformation|GetWorldLocation (Variables|Default|Getelevator)) (Transformation|GetActorLocation (Variables|Default|GettargetNode))))) (Variables|Default|GetcurSpeed)) (Transformation|GetWorldLocation (Variables|Default|Getelevator))) true)))
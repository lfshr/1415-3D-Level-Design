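; Small sliding door Blueprint that opens when something enters its trigger box and closes when it leaves.
; Box overlap plays or reverses a timeline that drives SetOpenAmount, which lowers the door mesh along Z by open amount times height unless locked in position.
; The construction script applies the same offset, so the placed door previews its open amount.
; EnableBrokenAnimation is an empty stub.
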(event OnComponentBeginOverlap(boxCollision)
  (params (OtherActor :type Actor%20Object%20Reference) (OtherComp :type Primitive%20Component%20Object%20Reference) (OtherBodyIndex :type Integer) (bFromSweep :type Boolean) (SweepResult :type Hit%20Result%20Structure%20%28by%20ref%29))
  (bind _openamount (Timeline|openCloseDoor Play)
    (:Update
      (CallFunction|SetOpenAmount _openamount))))

(event OnComponentEndOverlap(boxCollision)
  (params (OtherActor :type Actor%20Object%20Reference) (OtherComp :type Primitive%20Component%20Object%20Reference) (OtherBodyIndex :type Integer))
  (bind _openamount (Timeline|openCloseDoor Reverse)
    (:Update
      (CallFunction|SetOpenAmount _openamount))))

(event EventBeginPlay)

(event EventActorBeginOverlap
  (params (OtherActor :type Actor%20Object%20Reference)))

(event EventTick
  (params (DeltaSeconds :type Float%20%28single-precision%29)))

(fn ConstructionScript
  (Transformation|SetRelativeLocation (Variables|Default|Getdoor) (Math|Vector|MakeVector 0.0 0.0 (* (* (Variables|Default|GetopenAmount) (Variables|Default|Getheight)) -1.0)) false))

(fn SetOpenAmount
  (params (openAmount :type Float%20%28single-precision%29 :default 0.0))
  (if (not (Variables|Default|GetlockedInPosition))
    (bind _output_get (Variables|Default|SetopenAmount openAmount))
    (Transformation|SetRelativeLocation (Variables|Default|Getdoor) (Math|Vector|MakeVector 0.0 0.0 (* (* _output_get (Variables|Default|Getheight)) -1.0)) false)))

(fn EnableBrokenAnimation)
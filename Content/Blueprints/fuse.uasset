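; Fuse actor that a player can pick up and drop, shown as either an intact or blown mesh.
; The construction script picks the mesh from the default fuse type, and Break swaps it to blown through SetBroken.
; Overlapping the range sphere stores the player and enables input, so ActionPress toggles between attaching to the player and detaching with physics.
; Tick keeps a hologram above the fuse, with clamped pitch and zero roll.
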(event OnComponentEndOverlap(playerRangeSphere)
  (params (OtherActor :type Actor%20Object%20Reference) (OtherComp :type Primitive%20Component%20Object%20Reference) (OtherBodyIndex :type Integer))
  (if (== (Utilities|GetClass OtherActor) (Variables|Default|GetplayerClass))
    (Variables|Default|SetplayerInRange false)))

(event OnComponentBeginOverlap(playerRangeSphere)
  (params (OtherActor :type Actor%20Object%20Reference) (OtherComp :type Primitive%20Component%20Object%20Reference) (OtherBodyIndex :type Integer) (bFromSweep :type Boolean) (SweepResult :type Hit%20Result%20Structure%20%28by%20ref%29))
  (if (== (Utilities|GetClass OtherActor) (Variables|Default|GetplayerClass))
    (bind _aslevel_design_player (Utilities|Casting|CastToLevelDesignPlayer OtherActor))
    (Variables|Default|Setplayer _aslevel_design_player)
    (Input|EnableInput (Game|GetPlayerController _aslevel_design_player))
    (Variables|Default|SetplayerInRange true)))

(event EventBeginPlay)

(event EventActorBeginOverlap
  (params (OtherActor :type Actor%20Object%20Reference)))

(event EventTick
  (params (DeltaSeconds :type Float%20%28single-precision%29))
  (CallFunction|CalculateHologramLocation))

(event Input|ActionEvents|InputActionActionPress
  (:Pressed
    (if (Variables|Default|GetplayerInRange)
      (Development|PrintString "Hello")
      (CallFunction|PlayerPressed))))

(fn ConstructionScript
  (bind _defaultfuse (Variables|Default|GetdefaultFuse))
  (Utilities|FlowControl|Sequence
    (:then_0
      ;[1 1 1] Set Fuse Type
      (Variables|Default|SetcurrentFuse _defaultfuse)
      (if (Utilities|Enum|Equal(Enum) _defaultfuse "NewEnumerator0")
        (Components|StaticMesh|SetStaticMesh (Variables|Default|Getfuse) (Variables|Default|GetMAINFUSEMODEL))
        (elif (Utilities|Enum|Equal(Enum) _defaultfuse "NewEnumerator1")
          (Components|StaticMesh|SetStaticMesh (Variables|Default|Getfuse) (Variables|Default|GetBLOWNFUSEMODEL)))))
    (:then_1
      ;[1 1 1] Calculate hologram position
      (CallFunction|CalculateHologramLocation))
    (:then_2
      (Rendering|Material|SetMaterial (Variables|Default|Getfuse_hologram) 0 (Variables|Default|GetdefaultHologramMaterial)))))

(fn Break
  (CallFunction|SetBroken true))

(fn SetBroken
  (params (newValue :type Boolean :default false))
  (if newValue
    (Components|StaticMesh|SetStaticMesh (Variables|Default|Getfuse) (Variables|Default|GetBLOWNFUSEMODEL))
    (else
      (Components|StaticMesh|SetStaticMesh (Variables|Default|Getfuse) (Variables|Default|GetMAINFUSEMODEL)))))

(fn CalculateHologramLocation
  (bind _returnvalue (Transformation|GetActorRotation))
  (bind (_pitch _yaw) (Class|KismetMathLibrary|BreakRot _returnvalue))
  (Transformation|SetWorldTransform (Variables|Default|Getfuse_hologram) (Math|Transform|MakeTransform (+ (Transformation|GetActorLocation) (Math|Vector|MakeVector 0.0 0.0 (Variables|Default|GetholoGramDistance))) (Class|KismetMathLibrary|MakeRot (Math|Float|Clamp(Float) _pitch -5e+01 5e+01) _yaw 0.0)) false))

(fn PlayerPressed
  (bind _player (Variables|Default|Getplayer))
  (if (Variables|Default|Getattached)
    (Class|Actor|DetachRootComponentfromParent true)
    (Class|Actor|DetachRootComponentfromParent true)
    (Physics|SetSimulatePhysics true)
    (Variables|Default|Setattached false)
    (elif (!= _player 0)
      (Default|AttachActor _player self)
      (Variables|Default|Setattached true)
      (else
        (Development|PrintText "ERROR: Player is not set in fuse" true true "(R=1.000000,G=0.000000,B=0.085712,A=1.000000)")))))